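; Knight Blueprint holding a Resources map of names to amounts, with helper functions to add, remove, query, print and clear entries.
; AddResource stores only missing keys; it and RemoveResource print clamped totals without writing them back.
; ClearResources empties only the array returned by Values, leaving the map intact, while RemoveResourceType deletes the key.
; BeginPlay is empty, and the sample calls in the event graph are unwired.
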(event EventBeginPlay)

(fn ConstructionScript)

(fn AddResource
  (params (ResourceName :type String) (Amount :type Integer))
  (bind _resources (Variables|Default|GetResources))
  (bind (_value _returnvalue) (Utilities|Map|Find _resources ResourceName))
  (if _returnvalue
    _
    (else
      (Utilities|Map|Add _resources ResourceName Amount)))
  (Development|PrintString (Utilities|String|Append "Resource: " ResourceName "  Amount:  " (Utilities|String|ToString(Integer) (Math|Integer|Clamp(Integer) (+ _value Amount) 0 100)))))

(fn RemoveResource
  (params (ResourceName :type String) (Amount :type Integer))
  (bind _resources (Variables|Default|GetResources))
  (bind (_value _returnvalue) (Utilities|Map|Find _resources ResourceName))
  (if _returnvalue
    (Development|PrintString (Utilities|String|Append "Resource: " ResourceName "  Amount:  " (Utilities|String|ToString(Integer) (Math|Integer|Clamp(Integer) (- _value Amount) 0 100))))
    (else
      (Development|PrintString "0"))))

(fn GetResourceAmount
  (params (ResourceName%20 :type String))
  (bind _resources (Variables|Default|GetResources))
  (bind (_value _returnvalue) (Utilities|Map|Find _resources ResourceName%20))
  (if _returnvalue
    (Development|PrintString (Utilities|String|ToString(Integer) _value))
    (else
      (Development|PrintString "0"))))

(fn HasResource
  (params (ResourceName :type String))
  (return (Utilities|Map|Contains (Variables|Default|GetResources) ResourceName)))

(fn PrintResources
  (bind _resources (Variables|Default|GetResources))
  (bind _keys (Utilities|Map|Keys _resources))
  (for _array_element _keys
    (Development|PrintString (Utilities|String|Append "Resource: " _array_element " Amount: " (Utilities|String|ToString(Integer) (.Value (Utilities|Map|Find _resources _array_element)))))))

(fn RemoveResourceType
  (params (ResourceName :type String))
  (bind _resources (Variables|Default|GetResources))
  (if (.ReturnValue (Utilities|Map|Find _resources ResourceName))
    (Utilities|Map|Remove _resources ResourceName)))

(fn ClearResources
  (params (ResourceName :type String))
  (bind _resources (Variables|Default|GetResources))
  (if (.ReturnValue (Utilities|Map|Find _resources ResourceName))
    (bind _values (Utilities|Map|Values _resources))
    (Utilities|Array|Clear _values)))