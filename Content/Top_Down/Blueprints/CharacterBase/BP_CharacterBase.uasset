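; Top-down character base Blueprint that holds prototype resource, inventory, weapon and quest data, with debug output through PrintString.
; Helper functions work on a Resources map and struct arrays; resource amount changes are only printed, clamped to 0–100.
; CheckQuests matches required items to inventory names but marks only the standalone Quest variable completed.
; BeginPlay is empty, sample calls are unwired, and some totalling functions are stubs or incomplete.
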(event EventBeginPlay)

(fn ConstructionScript)

(fn AddResource
  (params (ResourceName :type String) (Amount :type Integer))
  (bind _resources (Variables|Resources|GetResources))
  (bind (_value _returnvalue) (Utilities|Map|Find _resources ResourceName))
  (if _returnvalue
    _
    (else
      (Utilities|Map|Add _resources ResourceName Amount)))
  (Development|PrintString (Utilities|String|Append "Resource: " ResourceName "  Amount:  " (Utilities|String|ToString(Integer) (Math|Integer|Clamp(Integer) (+ _value Amount) 0 100)))))

(fn RemoveResource
  (params (ResourceName :type String) (Amount :type Integer))
  (bind _resources (Variables|Resources|GetResources))
  (bind (_value _returnvalue) (Utilities|Map|Find _resources ResourceName))
  (if _returnvalue
    (Development|PrintString (Utilities|String|Append "Resource: " ResourceName "  Amount:  " (Utilities|String|ToString(Integer) (Math|Integer|Clamp(Integer) (- _value Amount) 0 100))))
    (else
      (Development|PrintString "0"))))

(fn PrintResources
  (bind _resources (Variables|Resources|GetResources))
  (bind _keys (Utilities|Map|Keys _resources))
  (for _array_element _keys
    (Development|PrintString (Utilities|String|Append "Resource: " _array_element " Amount: " (Utilities|String|ToString(Integer) (.Value (Utilities|Map|Find _resources _array_element)))))))

(fn HasResource
  (params (ResourceName :type String))
  (return (Utilities|Map|Contains (Variables|Resources|GetResources) ResourceName)))

(fn GetResourceAmount
  (params (ResourceName%20 :type String))
  (bind _resources (Variables|Resources|GetResources))
  (bind (_value _returnvalue) (Utilities|Map|Find _resources ResourceName%20))
  (if _returnvalue
    (Development|PrintString (Utilities|String|ToString(Integer) _value))
    (else
      (Development|PrintString "0"))))

(fn RemoveResourceType
  (params (ResourceName :type String))
  (bind _resources (Variables|Resources|GetResources))
  (if (.ReturnValue (Utilities|Map|Find _resources ResourceName))
    (Utilities|Map|Remove _resources ResourceName)))

(fn ClearResources
  (params (ResourceName :type String))
  (bind _resources (Variables|Resources|GetResources))
  (if (.ReturnValue (Utilities|Map|Find _resources ResourceName))
    (bind _values (Utilities|Map|Values _resources))
    (Utilities|Array|Clear _values)))

(fn ChangeItemValue
  (params (NewValue :type Integer))
  (Utilities|Struct|SetmembersinST_Item (Variables|Items|GetCurrentItem) NewValue))

(fn IsCurrentItemQuestItem
  (if (.isquestitem (Variables|Items|GetCurrentItem))
    (Development|PrintString "Yep!")
    (else
      (Development|PrintString "Nope!"))))

(fn PrintItemInfo
  (for _array_element (Variables|Items|GetInventory)
    (Development|PrintString (Utilities|String|Append "Item: " (.Name (Utilities|Struct|BreakST_Item _array_element)) " 
Description:" (.Description (Utilities|Struct|BreakST_Item _array_element)) " 
Value: " (Utilities|String|ToString(Integer) (.Value (Utilities|Struct|BreakST_Item _array_element))) " 
Weight:" (Utilities|String|ToString(Float) (.Weight (Utilities|Struct|BreakST_Item _array_element))) " 
Is a quest item: " (Utilities|String|ToString(Boolean) (.IsQuestItem (Utilities|Struct|BreakST_Item _array_element)))))))

(fn PrintWeaponInfo
  (bind _currentweapon (Variables|Weapons|GetCurrentWeapon))
  (Development|PrintString (Utilities|String|Append "Name: " (.name _currentweapon) " 
Damage:" (Utilities|String|ToString(Float) (.damage _currentweapon)) " 
AMMO: " (Utilities|String|ToString(Float) (.ammo _currentweapon)) " 
Is automatic: " (Utilities|String|ToString(Boolean) (.isautomatic _currentweapon)))))

(fn AddItem
  (params (NewItem :type ST%20Item%20Structure))
  (Utilities|Array|Add (Variables|Items|GetInventory) NewItem))

(fn FindItem
  (params (ItemName :type String))
  (if (Utilities|Array|ContainsItem (Variables|Items|GetInventory) (Utilities|Struct|MakeST_Item ItemName "" 0 0.0 false))
    (Development|PrintString "Found!")
    (else
      (Development|PrintString "Nope, not found!"))))

(fn CalculateInventoryValue
  (for _array_element (Variables|Items|GetInventory)
    _)
  (Development|PrintString (Utilities|String|Append "Total of values:  
" (Utilities|String|ToString(Integer) (+ (.value _array_element) 0))) true true "(R=0.000000,G=0.660000,B=1.000000,A=1.000000)" 1e+01))

(fn CalculateInventoryWeight)

(fn CheckQuests
  (for _array_element (Variables|Quests|GetActiveQuests)
    (for _array_element_2 (Variables|Items|GetInventory)
      (if (Utilities|Enum|Equal(Enum) (.name _array_element_2) (.requireditem _array_element))
        (bind _structout (Utilities|Struct|SetmembersinST_Quest (Variables|Quests|GetQuest) true))
        (Variables|Quests|SetQuest _structout)
        (Development|PrintString "Completed :)")
        (else
          (Development|PrintString "Not completed :("))))))

(fn GetCompletedQuestCount)

(fn AddQuest
  (params (NewQuest :type ST%20Quest%20Structure))
  (Utilities|Array|Add (Variables|Quests|GetActiveQuests) NewQuest))

(fn PrintQuestInfo
  (for _array_element (Variables|Quests|GetActiveQuests)
    (Development|PrintString (Utilities|String|Append "Quest name: " (.questname _array_element) " 
Quest description: " (.description _array_element) " 
Requiered Item: " (.requireditem _array_element) " 
EXP Reward: " (Utilities|String|ToString(Integer) (.reward _array_element)) " 
Is completed: " (Utilities|String|ToString(Boolean) (.completed _array_element))))))