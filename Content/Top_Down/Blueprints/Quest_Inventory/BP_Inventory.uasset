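; BP_Inventory is a simple inventory Blueprint that stores collected item names in the CollectedItems collection.
; Small functions add, remove, check, print, clear and count items, reporting results through PrintString rather than return values.
; BeginPlay exercises it as a smoke test by adding ItemName, printing the contents and checking that the item is present.
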(event EventBeginPlay
  (bind _item_name (Variables|Default|GetItem%20Name))
  (CallFunction|AddItem _item_name)
  (CallFunction|PrintInventory)
  (CallFunction|HasItem _item_name))

(fn ConstructionScript)

(fn AddItem
  (params (ItemName :type String))
  (Utilities|Array|Add (Variables|Default|GetCollectedItems) ItemName))

(fn RemoveItem
  (params (ItemName :type String))
  (Utilities|Array|RemoveItem (Variables|Default|GetCollectedItems) ItemName))

(fn HasItem
  (params (ItemName :type String))
  (if (Utilities|Array|ContainsItem (Variables|Default|GetCollectedItems) ItemName)
    (Development|PrintString "You have it!")
    (else
      (Development|PrintString "Nope, nothing here :("))))

(fn PrintInventory
  (for _array_element (Variables|Default|GetCollectedItems)
    (Development|PrintString _array_element)))

(fn ClearInventory
  (Utilities|Array|Clear (Variables|Default|GetCollectedItems)))

(fn GetItemCount
  (Development|PrintString (Utilities|String|ToString(Integer) (Utilities|Array|Length (Variables|Default|GetCollectedItems)))))