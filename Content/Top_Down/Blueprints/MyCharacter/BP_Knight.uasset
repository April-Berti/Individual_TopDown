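; Top-down player knight character with PaperZD animation, switchable between Idle, Melee and Ranged states through Enhanced Input.
; Movement runs along world X and Y and is blocked while an attack animation override plays, with its callbacks clearing the Attacking flag.
; Ranged attacks turn the knight toward the cursor hit point and spawn BP_Projectile along its forward vector; the cursor shows only in Ranged.
; Melee only plays its animation; Interact and NotifyAttack are empty.
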(event Input|EnhancedActionEvents|EnhancedInputActionIA_StateIdle
  (params (ActionValue :type Boolean) (ElapsedSeconds :type Float%20%28double-precision%29) (TriggeredSeconds :type Float%20%28double-precision%29) (InputAction :type Input%20Action%20Object%20Reference :default "/Game/Top_Down/Input/Action/IA_StateIdle.IA_StateIdle"))
  ;[0.15 0.15 0.15 0.5] States
  (:Started
    (Variables|Default|SetState "NewEnumerator0")
    (Variables|/Script/Engine.PlayerController|SetbShowMouseCursor (Game|GetPlayerController 0) false)))

(event Input|EnhancedActionEvents|EnhancedInputActionIA_Move
  (params (ActionValue :type Vector%202D%20Structure) (ElapsedSeconds :type Float%20%28double-precision%29) (TriggeredSeconds :type Float%20%28double-precision%29) (InputAction :type Input%20Action%20Object%20Reference :default "/Game/Top_Down/Input/Action/IA_Move.IA_Move"))
  ;[0.15 0.15 0.15 0.5] Movement
  (if (not (Variables|Default|GetAttacking))
    (Pawn|Input|AddMovementInput "1.000000,0.000000,0.000000" (.x ActionValue) false)
    (Pawn|Input|AddMovementInput "0.000000,1.000000,0.000000" (.y ActionValue) false)))

(event Input|EnhancedActionEvents|EnhancedInputActionIA_Attack
  (params (ActionValue :type Boolean) (ElapsedSeconds :type Float%20%28double-precision%29) (TriggeredSeconds :type Float%20%28double-precision%29) (InputAction :type Input%20Action%20Object%20Reference :default "/Game/Top_Down/Input/Action/IA_Attack.IA_Attack"))
  ;[0.15 0.15 0.15 0.5] Attacks
  (:Started
    (switch Utilities|FlowControl|Switch|SwitchonE_State (Variables|Default|GetState)
      (:NewEnumerator1
        (if (not (Variables|Default|GetAttacking))
          (|PlayAnimationOverridewithCallbacks (Variables|/Script/PaperZD.PaperZDAnimationComponent|GetAnimInstance (Variables|Default|GetAnimationComponent)) "/Game/Top_Down/Blueprints/MyCharacter/Animations/AnimSequences/SimpleAttack.SimpleAttack" "Simple_Attack" 1.0 0.0
            (:then
              (Variables|Default|SetAttacking true))
            (:OnCompleted
              (Variables|Default|SetAttacking false :!label _label))
            (:OnCancelled
              (goto _label)))))
      (:NewEnumerator2
        (if (not (Variables|Default|GetAttacking))
          (CallFunction|ShootProjectile)
          (|PlayAnimationOverridewithCallbacks (Variables|/Script/PaperZD.PaperZDAnimationComponent|GetAnimInstance (Variables|Default|GetAnimationComponent)) "/Game/Top_Down/Blueprints/MyCharacter/Animations/AnimSequences/DistantAttack.DistantAttack" "Distant_Attack" 1.0 0.0
            (:then
              (Variables|Default|SetAttacking true))
            (:OnCompleted
              (Variables|Default|SetAttacking false :!label _label_2))
            (:OnCancelled
              (goto _label_2))))))))

(event Input|EnhancedActionEvents|EnhancedInputActionIA_StateMelee
  (params (ActionValue :type Boolean) (ElapsedSeconds :type Float%20%28double-precision%29) (TriggeredSeconds :type Float%20%28double-precision%29) (InputAction :type Input%20Action%20Object%20Reference :default "/Game/Top_Down/Input/Action/IA_StateMelee.IA_StateMelee"))
  ;[0.15 0.15 0.15 0.5] States
  (:Started
    (Variables|Default|SetState "NewEnumerator1")
    (Variables|/Script/Engine.PlayerController|SetbShowMouseCursor (Game|GetPlayerController 0) false)))

(event Input|EnhancedActionEvents|EnhancedInputActionIA_StateRanged
  (params (ActionValue :type Boolean) (ElapsedSeconds :type Float%20%28double-precision%29) (TriggeredSeconds :type Float%20%28double-precision%29) (InputAction :type Input%20Action%20Object%20Reference :default "/Game/Top_Down/Input/Action/IA_StateRanged.IA_StateRanged"))
  ;[0.15 0.15 0.15 0.5] States
  (:Started
    (Variables|Default|SetState "NewEnumerator2")
    (Variables|/Script/Engine.PlayerController|SetbShowMouseCursor (Game|GetPlayerController 0) true)))

(event Input|EnhancedActionEvents|EnhancedInputActionIA_Interact
  (params (ActionValue :type Boolean) (ElapsedSeconds :type Float%20%28double-precision%29) (TriggeredSeconds :type Float%20%28double-precision%29) (InputAction :type Input%20Action%20Object%20Reference :default "/Game/Top_Down/Input/Action/IA_Interact.IA_Interact")))

(event EventBeginPlay
  ;[0.15 0.15 0.15 0.5] IMC
  (bind _asplayer_controller (Utilities|Casting|CastToPlayerController (Pawn|GetController)))
  (Input|AddMappingContext (PlayerController|LocalPlayerSubsystems|GetEnhancedInputLocalPlayerSubsystem _asplayer_controller) "/Game/Top_Down/Input/IMC/IMC_Move.IMC_Move" 0 "(bIgnoreAllPressedKeysUntilRelease=True,bForceImmediately=False,bNotifyUserSettings=False)"))

(event EventNotifyAttack
  ;[0.15 0.15 0.15 0.5] States
)

(fn ConstructionScript
  (|CallParentFunction))

(fn ShootProjectile
  (Transformation|SetActorRotation (Math|Rotator|MakeRotator 0.0 0.0 (.yaw (Math|Rotator|FindLookatRotation (Math|Vector|MakeVector 0.0 0.0 0.0) (- (.ImpactPoint (Collision|BreakHitResult (.HitResult (Game|Player|GetHitResultUnderCursorbyChannel (Game|GetPlayerController 0) "TraceTypeQuery1" true)))) (Transformation|GetActorLocation))))))
  (Game|SpawnActorfromClass "/Game/Top_Down/Blueprints/Fire_Projectile/BP_Projectile.BP_Projectile_C" (Transformation|GetActorTransform) "Undefined" "MultiplyWithRoot" 0 7e+02 (Transformation|GetActorForwardVector) 0))